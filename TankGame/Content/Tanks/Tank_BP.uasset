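; Player-controllable tank Blueprint that wires components together and routes input for driving, camera rotation and firing.
; On BeginPlay it passes the barrel and turret to TankAiming and both tracks to TankMovement.
; Driving input either sets each track's throttle directly or goes through TankMovement's move and turn intents.
; Aim axes rotate a separate yaw component and the spring arm's pitch, scaled by delta time, while the Fire action calls Fire.
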(event EventBeginPlay
  (Class|TankAimingComponent|Initalize (Variables|Default|GetTankAiming) (Variables|Default|GetBarrel) (Variables|Default|GetTankTurret))
  (Class|TankMovementComponent|Initalize (Variables|Default|GetTankMovement) (Variables|Default|GetLeftTrack) (Variables|Default|GetRightTrack)))

(event Input|ActionEvents|InputActionFire
  (params (Key :type Key%20Structure :default "AnyKey"))
  ;[1 1 1] Fireing stuff
  (:Pressed
    (Class|Tank|Fire)))

(event Input|AxisEvents|InputAxisAimX
  (params (AxisValue :type Float%20%28single-precision%29))
  ;[1 1 1] X Axis/Azimuth Camera Value
  (Transformation|AddLocalRotation (Variables|Default|GetXAxisRotation) (Math|Rotator|MakeRotator 0.0 0.0 (* AxisValue (Utilities|Time|GetWorldDeltaSeconds) 1e+02)) false false))

(event Input|AxisEvents|InputAxisMoveForward
  (params (AxisValue :type Float%20%28single-precision%29))
  ;[1 1 1] Movement Input Binding
  (Class|TankMovementComponent|IntendedMoveForward (Variables|Default|GetTankMovement) AxisValue))

(event Input|AxisEvents|InputAxisTurnRight
  (params (AxisValue :type Float%20%28single-precision%29))
  ;[1 1 1] Movement Input Binding
  (Class|TankMovementComponent|IntendedTurnRight (Variables|Default|GetTankMovement) AxisValue))

(event Input|AxisEvents|InputAxisAimY
  (params (AxisValue :type Float%20%28single-precision%29))
  ;[1 1 1] Y Axis Camera value
  (Transformation|AddLocalRotation (Variables|Default|GetSpringArm) (Math|Rotator|MakeRotator 0.0 (* AxisValue (Utilities|Time|GetWorldDeltaSeconds) 1e+02) 0.0) false false))

(event Input|AxisEvents|InputAxisLeftTrackThrottle
  (params (AxisValue :type Float%20%28single-precision%29))
  ;[1 1 1] Movement Input Binding
  (Class|TankTrack|SetThrottle (Variables|Default|GetLeftTrack) AxisValue))

(event Input|AxisEvents|InputAxisTurnLeft
  (params (AxisValue :type Float%20%28single-precision%29))
  ;[1 1 1] Movement Input Binding
  (Class|TankMovementComponent|IntendedTurnLeft (Variables|Default|GetTankMovement) AxisValue))

(event Input|AxisEvents|InputAxisRightTrackThrottle
  (params (AxisValue :type Float%20%28single-precision%29))
  ;[1 1 1] Movement Input Binding
  (Class|TankTrack|SetThrottle (Variables|Default|GetRightTrack) AxisValue))

(fn ConstructionScript)